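; Car Blueprint that spins its four wheels as it moves, without driving the movement itself.
; Tick adds the distance the first wheel travels in world space to a running total.
; That total becomes the relative pitch of all four wheels directly, with no radius conversion or direction sign.
; BeginPlay seeds the last location and also sets a non-looping timer by the name "Event Tick".
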(event `self.ReceiveBeginPlay`
  (`KismetSystemLibrary.K2_SetTimer` null "Event Tick" 0.1)
  (set `self.Last Location` (`SceneComponent.K2_GetComponentLocation` (`self.wheel`))))

(event `self.ReceiveTick`
  (params (DeltaSeconds :type "Float (single-precision)"))
  (bind _output_get (set `self.Distance Traveled` (+ (`KismetMathLibrary.VSize` (- (`SceneComponent.K2_GetComponentLocation` (`self.wheel`)) (`self.Last Location`))) (`self.Distance Traveled`))))
  (set `self.Last Location` (`SceneComponent.K2_GetComponentLocation` (`self.wheel`)))
  (`SceneComponent.K2_SetRelativeRotation` (`self.wheel`) (`KismetMathLibrary.MakeRotator` 0.0 _output_get) false false)
  (`SceneComponent.K2_SetRelativeRotation` (`self.wheel3`) (`KismetMathLibrary.MakeRotator` 0.0 _output_get) false false)
  (`SceneComponent.K2_SetRelativeRotation` (`self.wheel2`) (`KismetMathLibrary.MakeRotator` 0.0 _output_get) false false)
  (`SceneComponent.K2_SetRelativeRotation` (`self.wheel4`) (`KismetMathLibrary.MakeRotator` 0.0 _output_get) false false))

(fn `UserConstructionScript`)